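; BP_PuzzleBook is an interactable book that opens a color puzzle UI and rewards solving it with hint images.
; Its interact delegate plays a UI sound, spawns WBP_ColorPuzzle and binds to that widget's success event.
; On success it unbinds interaction, turns off repeat interaction and shows two timed WBP_Hint images in sequence, setting IsClear between them.
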(event Custom|OnInteractDelegate_Event
  (Audio|PlaySound2D "/Game/ProjectRD/Audio/Book_UI_Ver_2.Book_UI_Ver_2" 1.0 1.0 0.0 0 0)
  (bind _returnvalue (UserInterface|CreateWidget "/Game/ProjectRD/Widgets/WBP_ColorPuzzle.WBP_ColorPuzzle_C"))
  (bind _output_get (Variables|Default|SetPuzzleWidget _returnvalue))
  (UserInterface|Viewport|AddtoViewport _output_get 0)
  (EventDispatchers|AssignOnPuzzleSuccess _output_get (delegate Custom|OnPuzzleSuccess_Event)))

(event Custom|OnPuzzleSuccess_Event
  (EventDispatchers|UnbindEventfromOnInteractDelegate (delegate Custom|OnInteractDelegate_Event))
  (Variables|Default|SetbShouldRepeatInteraction false)
  (Class|BaseInteractableActor|CheckRepeat)
  (Utilities|FlowControl|Delay 1.5)
  (bind _returnvalue (CallFunction|ShowHindWidget "/Game/ProjectRD/Images/Dialogue/sc003.sc003"))
  (Utilities|FlowControl|Delay 3.0)
  (Widget|RemovefromParent _returnvalue)
  (Variables|Default|SetbIsClear true)
  (bind _returnvalue_2 (CallFunction|ShowHindWidget "/Game/ProjectRD/Images/Dialogue/sc004.sc004"))
  (Utilities|FlowControl|Delay 3.0)
  (Widget|RemovefromParent _returnvalue_2))

(event EventBeginPlay
  (EventDispatchers|AssignOnInteractDelegate (delegate Custom|OnInteractDelegate_Event)))

(event Collision|EventActorBeginOverlap
  (params (OtherActor :type Actor%20Object%20Reference)))

(event EventTick
  (params (DeltaSeconds :type Float%20%28single-precision%29)))

(fn ConstructionScript)

(fn ShowHindWidget
  (params (NewDialogueTexture :type Texture%202D%20Object%20Reference))
  (bind _returnvalue (UserInterface|CreateWidget "/Game/ProjectRD/Widgets/WBP_Hint.WBP_Hint_C"))
  (Class|BaseHintWidget|ChangeHintImage _returnvalue NewDialogueTexture)
  (UserInterface|Viewport|AddtoViewport _returnvalue 0)
  (return _returnvalue))