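; BP_SeqTriggerBox is a trigger actor that starts the game's ending when something overlaps it.
; On overlap it plays the ending music, locks input to game-only with no cursor or look input, and disables the player character's movement.
; It then plays the SQ_Ending level sequence and, after a fixed delay, adds the WBP_Ending widget to the viewport.
; The overlapping actor is not checked, and nothing guards against retriggering.
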(event EventBeginPlay
  (|CallParentFunction) ; This node is disabled and will not be called.\nDrag off pins to build functionality.
)

(event Collision|EventActorBeginOverlap
  (params (OtherActor :type Actor%20Object%20Reference))
  (bind _returnvalue (Game|GetPlayerController 0))
  (|CallParentFunction OtherActor)
  (Audio|PlaySound2D "/Game/ProjectRD/Sound/End/ENDBGM.ENDBGM" 1.0 1.0 0.0 0 0)
  ;[1 1 1] 시퀀서
  (Input|SetInputModeGameOnly _returnvalue false)
  (Variables|/Script/Engine.PlayerController|SetbShowMouseCursor _returnvalue false)
  (Input|SetIgnoreLookInput _returnvalue true)
  (bind _asbp_player_character (Utilities|Casting|CastToBP_PlayerCharacter (Game|GetPlayerCharacter 0)))
  (Pawn|Components|CharacterMovement|DisableMovement (Variables|/Script/Engine.Character|GetCharacterMovement _asbp_player_character))
  (bind _outactor (Sequencer|Player|CreateLevelSequencePlayer "/Game/Sequence/SQ_Ending.SQ_Ending"))
  (Sequencer|Player|Play (Variables|/Script/LevelSequence.LevelSequenceActor|GetSequencePlayer _outactor) :!class /Script/MovieScene.MovieSceneSequencePlayer)
  (Utilities|FlowControl|Delay 5.0)
  (bind _returnvalue_2 (UserInterface|CreateWidget "/Game/ProjectRD/Widgets/WBP_Ending.WBP_Ending_C"))
  (UserInterface|Viewport|AddtoViewport _returnvalue_2 0))

(event EventTick
  (params (DeltaSeconds :type Float%20%28single-precision%29))
  (|CallParentFunction DeltaSeconds) ; This node is disabled and will not be called.\nDrag off pins to build functionality.
)

(fn ConstructionScript
  (|CallParentFunction))